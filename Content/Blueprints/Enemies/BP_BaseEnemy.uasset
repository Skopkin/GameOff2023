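; Base enemy character that runs the BT_BaseEnemy behavior tree and can be killed by player projectiles.
; BeginPlay applies its walk speed and starts the tree on its AI controller.
; Overlapping a BP_PlayerProjectile subtracts that projectile's base damage from HP and destroys the projectile, and the enemy is destroyed at zero HP.
; RotateTowardsPlayer, not called within this Blueprint, yaws the enemy toward the player character.
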(event EventBeginPlay
  (Variables|/Script/Engine.CharacterMovementComponent|SetMaxWalkSpeed (Variables|Character|GetCharacterMovement) (Variables|Default|GetBase%20Movement%20Speed))
  (AI|RunBehaviorTree (AI|GetAIController self) "/Game/Blueprints/Enemies/BT_BaseEnemy.BT_BaseEnemy"))

(event Collision|EventActorBeginOverlap
  (params (OtherActor :type Actor%20Object%20Reference))
  (if (Utilities|ClassIsChildOf (Utilities|GetClass OtherActor) "/Game/Blueprints/Pickups/Weapons/Projectiles/BP_PlayerProjectile.BP_PlayerProjectile_C")
    (bind _asbp_player_projectile (Utilities|Casting|CastToBP_PlayerProjectile OtherActor))
    (CallFunction|TakeDamage (Variables|/Game/Blueprints/Pickups/Weapons/Projectiles/BP_BaseProjectile.BP_BaseProjectile_C|GetBase%20Damage _asbp_player_projectile))
    (Actor|DestroyActor _asbp_player_projectile)))

(event EventTick
  (params (DeltaSeconds :type Float%20%28single-precision%29)))

(fn ConstructionScript)

(fn RotateTowardsPlayer
  (bind _returnvalue (Pawn|GetControlRotation :!class /Script/Engine.Pawn))
  (Transformation|SetActorRotation (Math|Rotator|MakeRotator (.roll _returnvalue) (.pitch _returnvalue) (.yaw (Math|Rotator|FindLookatRotation (Transformation|GetActorLocation) (Transformation|GetActorLocation (Game|GetPlayerCharacter 0)))))))

(fn TakeDamage
  (params (Damage :type Float%20%28double-precision%29))
  (bind _output_get (Variables|Default|SetHP (- (Variables|Default|GetHP) Damage)))
  (if (<= _output_get 0.0)
    (Actor|DestroyActor)))