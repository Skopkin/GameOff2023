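; Ranged enemy Blueprint that runs a behavior tree and can fire projectiles at the player.
; On BeginPlay it calls the parent, then starts BT_RangedEnemy on its AI controller, printing an error if none is found.
; ShootProjectile calls RotateTowardsPlayer, then spawns a projectile at the actor's own transform.
; Overlap and Tick events are disabled stubs.
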(event EventBeginPlay
  (bind _self self)
  (bind _returnvalue (AI|GetAIController _self))
  (|CallParentFunction)
  (if (Utilities|IsValid _returnvalue)
    (AI|RunBehaviorTree _returnvalue "/Game/Blueprints/Enemies/BT_RangedEnemy.BT_RangedEnemy")
    (else
      (Development|PrintString "Can't find AI controller"))))

(event Collision|EventActorBeginOverlap
  (params (OtherActor :type Actor%20Object%20Reference))
  (|CallParentFunction OtherActor) ; This node is disabled and will not be called.\nDrag off pins to build functionality.
)

(event EventTick
  (params (DeltaSeconds :type Float%20%28single-precision%29))
  (|CallParentFunction DeltaSeconds) ; This node is disabled and will not be called.\nDrag off pins to build functionality.
)

(fn ConstructionScript
  (|CallParentFunction))

(fn ShootProjectile
  (CallFunction|RotateTowardsPlayer)
  (Game|SpawnActorfromClass (Variables|Default|GetProjectile) (Transformation|GetActorTransform) "Undefined" "MultiplyWithRoot" 0 0))