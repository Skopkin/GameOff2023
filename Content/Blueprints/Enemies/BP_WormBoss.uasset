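; BP_WormBoss is the worm boss enemy, whose health is shown on the main UI and whose destruction toggles the victory screen.
; On BeginPlay it runs the BT_WormBoss behavior tree, finds the MainUIWidget and shows a full boss health bar.
; Its TakeDamage override calls the parent, prints debug HP values and sends the HP fraction to the UI.
; On Destroyed it hides the boss UI.
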(event EventBeginPlay
  (|CallParentFunction)
  (AI|RunBehaviorTree (AI|GetAIController self) "/Game/Blueprints/Enemies/BT_WormBoss.BT_WormBoss")
  (bind _foundwidgets (Widget|GetAllWidgetsOfClass "/Game/UI/MainUIWidget.MainUIWidget_C" true))
  (bind _output_get (Variables|Default|SetUI (Utilities|Array|Get(acopy) _foundwidgets)))
  (Default|ToggleBossUI _output_get true)
  (Default|UpdateBossHP _output_get 1.0))

(event Collision|EventActorBeginOverlap
  (params (OtherActor :type Actor%20Object%20Reference))
  (|CallParentFunction OtherActor) ; This node is disabled and will not be called.\nDrag off pins to build functionality.
)

(event EventTick
  (params (DeltaSeconds :type Float%20%28single-precision%29))
  (|CallParentFunction DeltaSeconds) ; This node is disabled and will not be called.\nDrag off pins to build functionality.
)

(event EventDestroyed
  (bind _ui (Variables|Default|GetUI))
  (Default|ToggleBossUI _ui false)
  (Default|ToggleVictoryScreen _ui))

(fn ConstructionScript
  (|CallParentFunction))

(fn TakeDamage
  (params (Damage :type Integer))
  (bind _max_hp (Variables|Default|GetMax%20HP))
  (bind _hp (Variables|Default|GetHP))
  (bind _returnvalue (Math|Conversions|ToFloat(Integer) _max_hp))
  (bind _returnvalue_2 (Math|Conversions|ToFloat(Integer) _hp))
  (bind _returnvalue_3 (/ _returnvalue_2 _returnvalue))
  (|CallParentFunction Damage)
  (Development|PrintString (Utilities|String|Append (Utilities|String|ToString(Integer) _hp) " / " (Utilities|String|ToString(Integer) _max_hp)))
  (Development|PrintString (Utilities|String|Append (Utilities|String|ToString(Float) _returnvalue_3) "%"))
  (Default|UpdateBossHP (Variables|Default|GetUI) _returnvalue_3))