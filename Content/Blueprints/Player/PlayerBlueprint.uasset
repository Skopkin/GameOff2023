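; Player character Blueprint with cursor-aimed attacks, world-axis movement and a swappable one-weapon, one-ability inventory.
; Primary attack turns toward a mouse trace, then advances a melee combo with slowed walking or spawns the ranged weapon's projectile.
; Pickups are stored as hidden actors, and the replaced item respawns in front.
; Enemy overlaps cause damage, camera shake and UI updates; abilities, secondary attacks and death are print-only or unwired stubs.
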(event Custom|PickUpItemEvent
  (params (PickupStruct :type S%20Pickup%20Structure) (Pickup%20Class :type BP%20Pickup%20Class%20Reference))
  (bind _inventory (Variables|Default|GetInventory))
  ;[1 1 1] Pick Up
  (switch Utilities|FlowControl|Switch|SwitchonE_PickupType (.Type (Utilities|Struct|BreakS_Pickup PickupStruct))
    (:NewEnumerator0
      (CallFunction|HandleWeaponPickup (.weapon _inventory) Pickup%20Class))
    (:NewEnumerator1
      (CallFunction|HandleAbilityPickup (.ability _inventory) Pickup%20Class))))

(event Input|EnhancedActionEvents|EnhancedInputActionIA_Move
  (params (ActionValue :type Vector%202D%20Structure) (ElapsedSeconds :type Float%20%28double-precision%29) (TriggeredSeconds :type Float%20%28double-precision%29) (InputAction :type Input%20Action%20Object%20Reference :default "/Game/Inputs/IA_Move.IA_Move"))
  ;[1 1 1] Movement
  (:Triggered
    (Pawn|Input|AddMovementInput "0.000000,1.000000,0.000000" (.x ActionValue) false)
    (Pawn|Input|AddMovementInput "1.000000,0.000000,0.000000" (.y ActionValue) false)))

(event Input|EnhancedActionEvents|EnhancedInputActionIA_PrimaryAttack
  (params (ActionValue :type Vector%202D%20Structure) (ElapsedSeconds :type Float%20%28double-precision%29) (TriggeredSeconds :type Float%20%28double-precision%29) (InputAction :type Input%20Action%20Object%20Reference :default "/Game/Inputs/IA_PrimaryAttack.IA_PrimaryAttack"))
  (bind _inventory (Variables|Default|GetInventory))
  ;[1 1 1] Primary Attack
  (:Started
    (if (Utilities|IsValid (.weapon _inventory))
      (CallFunction|RotateTowardsCursor)
      (switch Utilities|FlowControl|Switch|SwitchonE_WeaponType (.weapontype (Variables|/Game/Blueprints/Pickups/Weapons/BP_Weapon.BP_Weapon_C|GetBase%20Weapon%20Properties (.weapon _inventory)))
        (:NewEnumerator0
          (Variables|/Script/Engine.CharacterMovementComponent|SetMaxWalkSpeed (Variables|Character|GetCharacterMovement) (Variables|Default|GetAttack%20Walk%20Speed))
          (bind _continue_combo (CallFunction|HandleMeleePrimaryAttack))
          (if _continue_combo
            (Utilities|FlowControl|Delay 1.0)
            (Variables|/Script/Engine.CharacterMovementComponent|SetMaxWalkSpeed (Variables|Character|GetCharacterMovement) (Variables|Default|GetMax%20Walk%20Speed))
            (Variables|Default|SetCombo%20Counter 0)
            (Development|PrintString "Reset")))
        (:NewEnumerator1
          (CallFunction|HandleRangedAttack)))
      (else
        (Development|PrintString "No Weapon Equipped")))))

(event Input|EnhancedActionEvents|EnhancedInputActionIA_SecondaryAttack
  (params (ActionValue :type Vector%202D%20Structure) (ElapsedSeconds :type Float%20%28double-precision%29) (TriggeredSeconds :type Float%20%28double-precision%29) (InputAction :type Input%20Action%20Object%20Reference :default "/Game/Inputs/IA_SecondaryAttack.IA_SecondaryAttack"))
  ;[1 1 1] Secondary Attack
)

(event Input|EnhancedActionEvents|EnhancedInputActionIA_ActivateAbility
  (params (ActionValue :type Vector%202D%20Structure) (ElapsedSeconds :type Float%20%28double-precision%29) (TriggeredSeconds :type Float%20%28double-precision%29) (InputAction :type Input%20Action%20Object%20Reference :default "/Game/Inputs/IA_ActivateAbility.IA_ActivateAbility"))
  (bind _inventory (Variables|Default|GetInventory))
  ;[1 1 1] Ability
  (:Started
    (if (Utilities|IsValid (.ability _inventory))
      (Development|PrintString (Utilities|String|Append (.name (Variables|/Game/Blueprints/Pickups/BP_Pickup.BP_Pickup_C|GetPickup%20Properties (.ability _inventory))) " used"))
      (else
        (Development|PrintString "No ability equipped")))))

(event EventBeginPlay
  ;[1 1 1] On Start
  (Utilities|FlowControl|Sequence
    (:then_0
      (CallFunction|MapInputs)
      (Variables|/Script/Engine.PlayerController|SetbShowMouseCursor (Game|GetPlayerController 0) true)
      (bind _returnvalue (UserInterface|CreateWidget "/Game/UI/MainUIWidget.MainUIWidget_C" (Game|GetPlayerController 0)))
      (bind _output_get (Variables|Default|SetUI _returnvalue))
      (UserInterface|Viewport|AddtoViewport _output_get 0)
      (Class|Pawn|SetCanAffectNavigationGeneration self false))))

(event Collision|EventActorBeginOverlap
  (params (OtherActor :type Actor%20Object%20Reference))
  (bind _returnvalue (Utilities|GetClass OtherActor))
  (if (Utilities|ClassIsChildOf _returnvalue "/Game/Blueprints/Pickups/Weapons/Projectiles/BP_EnemyProjectile.BP_EnemyProjectile_C")
    (bind _asbp_enemy_projectile (Utilities|Casting|CastToBP_EnemyProjectile OtherActor))
    (CallFunction|TakeDamage (Variables|/Game/Blueprints/Pickups/Weapons/Projectiles/BP_BaseProjectile.BP_BaseProjectile_C|GetBase%20Damage _asbp_enemy_projectile) "/Game/Effects/CameraShake/MediumCamShake.MediumCamShake_C")
    (Actor|DestroyActor _asbp_enemy_projectile)
    (elif (Utilities|ClassIsChildOf _returnvalue "/Game/Blueprints/Enemies/BP_BaseEnemy.BP_BaseEnemy_C")
      (bind _asbp_base_enemy (Utilities|Casting|CastToBP_BaseEnemy OtherActor))
      (Character|LaunchCharacter (* (Math|Vector|GetUnitDirection(Vector) (Transformation|GetActorLocation _asbp_base_enemy) (Transformation|GetActorLocation)) (Variables|/Game/Blueprints/Enemies/BP_BaseEnemy.BP_BaseEnemy_C|GetKnockback%20Value _asbp_base_enemy)) true false)
      (CallFunction|TakeDamage 1 "/Game/Effects/CameraShake/LargeCamShake.LargeCamShake_C"))))

(event EventTick
  (params (DeltaSeconds :type Float%20%28single-precision%29))
  (Class|Pawn|ConsumeMovementInputVector))

(fn ConstructionScript)

(fn MapInputs
  (bind _asplayer_controller (Utilities|Casting|CastToPlayerController (Game|GetPlayerController 0)))
  (Utilities|IsValid (PlayerController|LocalPlayerSubsystems|GetEnhancedInputLocalPlayerSubsystem _asplayer_controller)
    (:Is%20Valid
      (Input|AddMappingContext (PlayerController|LocalPlayerSubsystems|GetEnhancedInputLocalPlayerSubsystem _asplayer_controller) "/Game/Inputs/IAC_PlayerController.IAC_PlayerController" 0 "(bIgnoreAllPressedKeysUntilRelease=True,bForceImmediately=False)"))))

(fn DropWeapon
  (params (Current%20Weapon%20Actor :type BP%20Pickup%20Class%20Reference))
  (bind _returnvalue (Game|SpawnActorfromClass Current%20Weapon%20Actor (Math|Transform|MakeTransform (Transformation|GetWorldLocation (Variables|Default|GetForward%20Arrow)) "0.000000,180.000000,0.000000" "1.000000,1.000000,1.000000") "Undefined" "MultiplyWithRoot" 0 0)))

(fn StoreWeapon
  (params (New%20Weapon%20Class :type BP%20Pickup%20Class%20Reference))
  (bind _returnvalue (Game|SpawnActorfromClass New%20Weapon%20Class (Math|Transform|MakeTransform (Transformation|GetWorldLocation (Variables|Default|GetForward%20Arrow)) "0, 0, 0" "1.000000,1.000000,1.000000") "Undefined" "MultiplyWithRoot" 0 0))
  (bind _asbp_weapon (Utilities|Casting|CastToBP_Weapon _returnvalue))
  (Rendering|SetActorHiddenInGame _asbp_weapon true)
  (Collision|SetCollisionEnabled (Variables|/Game/Blueprints/Pickups/BP_Pickup.BP_Pickup_C|GetSphere _asbp_weapon) "NoCollision")
  (Variables|Default|SetInventory (Utilities|Struct|MakeS_PlayerInventory _asbp_weapon (.ability (Variables|Default|GetInventory)))))

(fn DropAbility
  (params (Current%20Ability%20Actor :type BP%20Pickup%20Class%20Reference))
  (Development|PrintString (Utilities|String|Append "Dropped " (Utilities|GetClassDisplayName Current%20Ability%20Actor)))
  (Game|SpawnActorfromClass Current%20Ability%20Actor (Math|Transform|MakeTransform (Transformation|GetWorldLocation (Variables|Default|GetForward%20Arrow)) "0.000000,180.000000,0.000000" "1.000000,1.000000,1.000000") "Undefined" "MultiplyWithRoot" 0 0))

(fn StoreAbility
  (params (New%20Ability%20Class :type BP%20Pickup%20Class%20Reference))
  (bind _returnvalue (Game|SpawnActorfromClass New%20Ability%20Class (Math|Transform|MakeTransform (Transformation|GetWorldLocation (Variables|Default|GetForward%20Arrow)) "0, 0, 0" "1.000000,1.000000,1.000000") "Undefined" "MultiplyWithRoot" 0 0))
  (bind _asbp_ability (Utilities|Casting|CastToBP_Ability _returnvalue))
  (Rendering|SetActorHiddenInGame _asbp_ability true)
  (Collision|SetCollisionEnabled (Variables|/Game/Blueprints/Pickups/BP_Pickup.BP_Pickup_C|GetSphere _asbp_ability) "NoCollision")
  (Variables|Default|SetInventory (Utilities|Struct|MakeS_PlayerInventory (.weapon (Variables|Default|GetInventory)) _asbp_ability))
  (Development|PrintString (Utilities|String|Append "Picked up " (Utilities|GetClassDisplayName New%20Ability%20Class))))

(fn HandleAbilityPickup
  (params (Current%20Ability%20Actor :type BP%20Ability%20Object%20Reference) (New%20Ability%20Class :type BP%20Pickup%20Class%20Reference))
  (if (Utilities|IsValid Current%20Ability%20Actor)
    (CallFunction|DropAbility (Utilities|GetClass Current%20Ability%20Actor))
    (Actor|DestroyActor Current%20Ability%20Actor))
  (CallFunction|StoreAbility New%20Ability%20Class))

(fn HandleWeaponPickup
  (params (Equipped%20Weapon :type BP%20Weapon%20Object%20Reference) (New%20Weapon :type BP%20Pickup%20Class%20Reference))
  (if (Utilities|IsValid Equipped%20Weapon)
    (CallFunction|DropWeapon (Utilities|GetClass Equipped%20Weapon))
    (Actor|DestroyActor Equipped%20Weapon))
  (CallFunction|StoreWeapon New%20Weapon))

(fn GetWeaponType
  (bind _inventory (Variables|Default|GetInventory))
  (if (Utilities|IsValidClass (.weapon _inventory))
    (switch Utilities|FlowControl|Switch|SwitchonE_WeaponType "NewEnumerator0"
      (:NewEnumerator0
        (Utilities|Casting|CastToBP_Weapon_MeleeClass (.weapon _inventory)))
      (:NewEnumerator1
        (Utilities|Casting|CastToBP_Weapon_RangedClass (.weapon _inventory))))
    (else
      (Development|PrintString "No Weapon Equipped"))))

(fn HandleMeleePrimaryAttack
  (bind _asbp_weapon_melee (Utilities|Casting|CastToBP_Weapon_Melee (.weapon (Variables|Default|GetInventory))))
  (if (< (Variables|Default|GetCombo%20Counter) (.maxcombo (Variables|/Game/Blueprints/Pickups/Weapons/BP_Weapon_Melee.BP_Weapon_Melee_C|GetMelee%20Properties _asbp_weapon_melee)))
    (bind _output_get (Variables|Default|SetCombo%20Counter (+ (Variables|Default|GetCombo%20Counter) 1)))
    (Development|PrintString (Utilities|String|Append (.name (Variables|/Game/Blueprints/Pickups/BP_Pickup.BP_Pickup_C|GetPickup%20Properties _asbp_weapon_melee)) (Utilities|String|ToString(Integer) _output_get)))
    (return true)
    (else
      (Development|PrintString "Combo Finish!")
      (return false))))

(fn HandleRangedAttack
  (bind _self self)
  (bind _returnvalue (Transformation|GetActorTransform _self))
  (bind _asbp_weapon_ranged (Utilities|Casting|CastToBP_Weapon_Ranged (.weapon (Variables|Default|GetInventory))))
  (Game|SpawnActorfromClass (.projectile (Variables|/Game/Blueprints/Pickups/Weapons/BP_Weapon_Ranged.BP_Weapon_Ranged_C|GetRanged%20Properties _asbp_weapon_ranged)) (Math|Transform|MakeTransform (.location _returnvalue) (.rotation _returnvalue) "1.000000,1.000000,1.000000") "Undefined" "MultiplyWithRoot" 0 0))

(fn HandleMeleeSecondaryAttack
  (bind _asbp_weapon_melee (Utilities|Casting|CastToBP_Weapon_Melee (.weapon (Variables|Default|GetInventory))))
  (Development|PrintString (Utilities|String|Append (.name (Variables|/Game/Blueprints/Pickups/BP_Pickup.BP_Pickup_C|GetPickup%20Properties _asbp_weapon_melee)) " secondary attack")))

(fn HandleRangedSecondaryAttack
  (bind _asbp_weapon_ranged (Utilities|Casting|CastToBP_Weapon_Ranged (.weapon (Variables|Default|GetInventory))))
  (Development|PrintString (Utilities|String|Append (.name (Variables|/Game/Blueprints/Pickups/BP_Pickup.BP_Pickup_C|GetPickup%20Properties _asbp_weapon_ranged)) " secondary attack")))

(fn RotateTowardsCursor
  (bind _returnvalue (Game|GetPlayerController 0))
  (bind _returnvalue_2 (Transformation|GetActorRotation))
  (bind (_worldlocation _worlddirection) (Game|Player|ConvertMouseLocationToWorldSpace _returnvalue))
  (bind _outhit (Collision|LineTraceByChannel _worldlocation (+ _worldlocation (* _worlddirection 5e+05)) "TraceTypeQuery1" false 0 "ForOneFrame"))
  (Transformation|SetActorRotation (Math|Rotator|MakeRotator (.roll _returnvalue_2) (.pitch _returnvalue_2) (.yaw (Math|Rotator|FindLookatRotation (Transformation|GetActorLocation) (.location _outhit))))))

(fn TakeDamage
  (params (Damage :type Integer) (Camera%20Shake%20Size :type Legacy%20Camera%20Shake%20Class%20Reference))
  (bind _ui (Variables|Default|GetUI))
  (Camera|PlayWorldCameraShake Camera%20Shake%20Size (Transformation|GetActorLocation) 0.0 1e+07)
  (bind _output_get (Variables|Default|SetCurrent%20HP (- (Variables|Default|GetCurrent%20HP) Damage)))
  (if (> _output_get 0)
    (Default|UpdateSuns _ui _output_get)
    (else
      (Default|UpdateSuns _ui)
      (Development|PrintString "DED"))))