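; Inventory item actor that carries a 2D grid footprint stored as a flattened array.
; The construction script has GameModeBlueprint build the grid array from GridSize and GridProg via MakeInventoryArray.
; RotateItemGrid swaps the X and Y size and remaps cells with transpose-and-flip index math for a quarter turn, returning GridArr.
; The event graph holds only disabled placeholder events.
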(event EventBeginPlay)

(event Collision|EventActorBeginOverlap
  (params (OtherActor :type Actor%20Object%20Reference)))

(event EventTick
  (params (DeltaSeconds :type Float%20%28single-precision%29)))

(fn ConstructionScript
  (bind _asgame_mode_blueprint (Utilities|Casting|CastToGameModeBlueprint (Game|GetGameMode)))
  (Default|MakeInventoryArray _asgame_mode_blueprint (Variables|Default|GetgridArr) (Variables|Default|GetgridSize) (Variables|Default|GetgridProg)))

(fn RotateItemGrid
  (bind _array (Utilities|Array|MakeArray))
  (bind _output_get (Variables|Default|SetgridSize (Math|Vector|MakeVector (.y (Variables|Default|GetgridSize)) (.x (Variables|Default|GetgridSize)) (.z (Variables|Default|GetgridSize))))) ; Swap grid size
  (bind _asgame_mode_blueprint (Utilities|Casting|CastToGameModeBlueprint (Game|GetGameMode)))
  (Default|MakeInventoryArray _asgame_mode_blueprint _array _output_get (Utilities|Array|MakeArray))
  (for _index (range 0 (Math|Float|Truncate (.x (Variables|Default|GetgridSize)))) ; i
    (for _index_2 (range 0 (Math|Float|Truncate (.y (Variables|Default|GetgridSize)))) ; j
      (Utilities|Array|SetArrayElem _array (Utilities|CoordtoIndex (Math|Float|Truncate (.x (Variables|Default|GetgridSize))) _index_2 (Utilities|Operators|Subtract (Math|Float|Truncate (.y (Variables|Default|GetgridSize))) 1 _index)) (Utilities|Array|Get(acopy) (Variables|Default|GetgridArr) (Utilities|CoordtoIndex (Math|Float|Truncate (.x (Variables|Default|GetgridSize))) _index _index_2)))))
  (bind _output_get_2 (Variables|Default|SetgridArr _array))
  (return _output_get_2))