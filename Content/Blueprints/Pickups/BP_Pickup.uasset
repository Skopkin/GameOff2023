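; BP_Pickup is a world item that the player collects by pressing E while standing inside its sphere.
; Sphere overlap with a PlayerBlueprint toggles the actor's input on player controller 0 and shows or clears a context label naming the item.
; Pressing E passes the pickup's properties struct and class to the player's PickUpItemEvent, then destroys the actor.
; On BeginPlay the actor resets its rotation to zero.
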(event OnComponentBeginOverlap(Sphere)
  (params (OverlappedComponent :type Primitive%20Component%20Object%20Reference) (OtherActor :type Actor%20Object%20Reference) (OtherComp :type Primitive%20Component%20Object%20Reference) (OtherBodyIndex :type Integer) (bFromSweep :type Boolean) (SweepResult :type Hit%20Result%20Structure%20%28by%20ref%29))
  (Utilities|Casting|CastToPlayerBlueprint OtherActor)
  (Input|EnableInput (Game|GetPlayerController 0))
  (Rendering|Components|TextRender|SetText (Variables|Default|GetContextLabel) (Utilities|Text|ToText(String) (Utilities|String|Append "Pickup: " (.Name (Utilities|Struct|BreakS_Pickup (Variables|Default|GetPickup%20Properties)))))))

(event OnComponentEndOverlap(Sphere)
  (params (OverlappedComponent :type Primitive%20Component%20Object%20Reference) (OtherActor :type Actor%20Object%20Reference) (OtherComp :type Primitive%20Component%20Object%20Reference) (OtherBodyIndex :type Integer))
  (Utilities|Casting|CastToPlayerBlueprint OtherActor)
  (Input|DisableInput (Game|GetPlayerController 0))
  (Rendering|Components|TextRender|SetText (Variables|Default|GetContextLabel) (Utilities|Text|ToText(String) "")))

(event EventBeginPlay
  (Transformation|SetActorRotation "0, 0, 0" true))

(event Input|KeyboardEvents|E
  (params (Key :type Key%20Structure :default "None"))
  (:Pressed
    (bind _asplayer_blueprint (Utilities|Casting|CastToPlayerBlueprint (stale OnComponentBeginOverlap(Sphere) OtherActor)))
    (Default|PickUpItemEvent _asplayer_blueprint (Variables|Default|GetPickup%20Properties) (Utilities|GetClass self))
    (Development|PrintString "Destroying item")
    (Actor|DestroyActor)))

(fn ConstructionScript)